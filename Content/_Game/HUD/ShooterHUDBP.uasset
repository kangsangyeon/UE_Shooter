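; Shooter HUD Blueprint that draws a crosshair on screen using immediate-mode canvas drawing.
; On DrawHUD, it computes the screen center and adds a configurable location offset.
; It draws the crosshair texture at its native size, shifted back by half its width and height to center it on that point.
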(event EventDrawHUD
  (params (SizeX :type Integer) (SizeY :type Integer))
  (bind _crosshairtexture (Variables|Default|GetCrosshairTexture))
  (Variables|Default|SetScreenCenter (Math|Vector2D|MakeVector2D (Math|Conversions|ToFloat(Integer) (/ SizeX 2)) (Math|Conversions|ToFloat(Integer) (/ SizeY 2))))
  (Variables|Default|SetCrosshairTextureWidth (Class|Texture2D|BlueprintGetSizeX _crosshairtexture))
  (Variables|Default|SetCrosshairTextureHeight (Class|Texture2D|BlueprintGetSizeY _crosshairtexture))
  (Canvas|DrawTexture (Variables|Default|GetCrosshairTexture) (- (.X (Math|Vector2D|BreakVector2D (+ (Variables|Default|GetScreenCenter) (Variables|Default|GetCrosshairLocationOffset)))) (Math|Conversions|ToFloat(Integer) (/ (Variables|Default|GetCrosshairTextureWidth) 2))) (- (.Y (Math|Vector2D|BreakVector2D (+ (Variables|Default|GetScreenCenter) (Variables|Default|GetCrosshairLocationOffset)))) (Math|Conversions|ToFloat(Integer) (/ (Variables|Default|GetCrosshairTextureHeight) 2))) (Math|Conversions|ToFloat(Integer) (Variables|Default|GetCrosshairTextureWidth)) (Math|Conversions|ToFloat(Integer) (Variables|Default|GetCrosshairTextureHeight)) 0.0 0.0 1.0 1.0 "(R=1.000000,G=1.000000,B=1.000000,A=1.000000)"))

(fn ConstructionScript)